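; BP_ProspectorDataDeposit is a hackable objective building, by its name the data deposit tied to the Prospector.
; It is a thin child Blueprint: BeginPlay, construction, hacking completion and widget class lookup all defer to the parent.
; SpawnDataCell and the load, overcharger and generator-connection handlers are empty stubs, and Tick and overlap are disabled, so this graph adds no logic of its own.
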(event `self.ReceiveBeginPlay`
  (`parent.ReceiveBeginPlay`))

(event `OnLoaded_B91065F0477C87A6C355AF868F6F6BB2`
  (params (Loaded :type "Object Class Reference")))

(event `OnOverChargerCalled_Event_0`
  (params (Location :type "Vector Structure") (RoomIndex :type Integer)))

(event `FirstConnect_Event`
  (params (Generator :type "/Game/GameElements/Objectives/Facility/ShieldGenerator/BP_Facility_PowerStation_GeneratorBase Object Reference") (tetherlineStart :type "TetherComponent Object Reference")))

(event `self.OnHackingComplete`
  (`parent.OnHackingComplete`))

(fn `GetWidgetClass`
  (returns (ReturnValue :type "BossFightWidget Class Reference"))
  (bind _returnvalue (`parent.GetWidgetClass`))
  (return _returnvalue))

(fn `SpawnDataCell`)

(fn `UserConstructionScript`
  (`parent.UserConstructionScript`))