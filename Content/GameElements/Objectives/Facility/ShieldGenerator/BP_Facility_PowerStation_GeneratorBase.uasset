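; BP_Facility_PowerStation_GeneratorBase is a base Blueprint for a power station generator in the Facility shield generator objective.
; BeginPlay and the hacking completion and change events only forward to the parent class.
; Hooks for the overcharger call, match start, room assignment, replicated hacking pod, power and discovery state, and getters for connector, boss and widget are empty stubs.
; IsStillValid always returns false.
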(event `self.ReceiveBeginPlay`
  (`parent.ReceiveBeginPlay`))

(event `Cheat_CallOverCharger`)

(event `OnMatchStarted_Event_0`)

(event `self.OnHackingComplete`
  (`parent.OnHackingComplete`))

(event `self.OnHackingChanged`
  (params (NewIsHacking :type Boolean))
  (`parent.OnHackingChanged` NewIsHacking))

(fn `GetBossActor`
  (returns (ReturnValue :type "Actor Object Reference"))
  (return null))

(fn `GetCallOverchargerUsable`
  (returns (Usable :type "SingleUsableComponent Object Reference"))
  (return null))

(fn `GetConnectorPoint`
  (returns (OutTransform :type "Array of Transform Structure"))
  (return))

(fn `GetWidgetClass`
  (returns (ReturnValue :type "BossFightWidget Class Reference"))
  (return null))

(fn `IsStillValid`
  (returns (ReturnValue :type Boolean))
  (return false))

(fn `OnRep_ConnectedHackingPod`)

(fn `OnRep_Discovered`)

(fn `OnRep_HackingPower`)

(fn `SetRoom`
  (params (RoomIndex :type Integer)))

(fn `UserConstructionScript`)