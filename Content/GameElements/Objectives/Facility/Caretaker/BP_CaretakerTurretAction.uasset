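; Caretaker action Blueprint for the Facility objective, named for a turret attack but containing only skeleton logic.
; OnStarted, OnStopped, OnTriggered and CanUse simply defer to the parent class.
; Events for turret waves, spawning and death, drone setup and light toggling are empty stubs, so this asset adds no behavior of its own.
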(event `self.OnStarted`
  (`parent.OnStarted`))

(event `Turret wave`)

(event `self.OnStopped`
  (`parent.OnStopped`))

(event `SetupDrone`
  (params (drone :type "/Game/GameElements/Objectives/Facility/DefenseTurret/BP_FacilityTurretDrone Object Reference") (transform :type "Transform Structure")))

(event `TurretSpawned`
  (params (spawnedTurret :type "FacilityTurret Object Reference")))

(event `TurretDied`
  (params (HealthComponent :type "HealthComponentBase Object Reference")))

(event `self.OnTriggered`
  (`parent.OnTriggered`))

(event `SpawnTurrets`
  (params (amountOfTurrets :type Integer)))

(event `ActivateLights`)

(event `DeactivateLights`)

(fn `CanUse`
  (returns (ReturnValue :type Boolean))
  (return (`parent.CanUse`)))